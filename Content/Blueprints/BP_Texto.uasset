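; BP_Texto is a readable note actor that shows a diary widget when the player interacts with it.
; Interactuar toggles reading through the Estaleyendo flag, creating BP_widgetDiario on pickup and removing it on put down.
; A Box trigger shows an InterfazInterraccion widget while BP_FirstPersonCharacter overlaps it and removes it when the overlap ends.
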(event OnComponentEndOverlap(Box)
  (params (OverlappedComponent :type Primitive%20Component%20Object%20Reference) (OtherActor :type Actor%20Object%20Reference) (OtherComp :type Primitive%20Component%20Object%20Reference) (OtherBodyIndex :type Integer))
  (Utilities|Casting|CastToBP_FirstPersonCharacter OtherActor)
  (Widget|RemovefromParent (stale OnComponentBeginOverlap(Box) _returnvalue)))

(event OnComponentBeginOverlap(Box)
  (params (OverlappedComponent :type Primitive%20Component%20Object%20Reference) (OtherActor :type Actor%20Object%20Reference) (OtherComp :type Primitive%20Component%20Object%20Reference) (OtherBodyIndex :type Integer) (bFromSweep :type Boolean) (SweepResult :type Hit%20Result%20Structure%20%28by%20ref%29))
  (Utilities|Casting|CastToBP_FirstPersonCharacter OtherActor)
  (bind _returnvalue (UserInterface|CreateWidget "/Game/Blueprints/InterfazInterraccion.InterfazInterraccion_C"))
  (UserInterface|Viewport|AddtoViewport _returnvalue 0))

(event Custom|PutDownNote
  (Widget|RemovefromParent (stale Custom|PickupNote _returnvalue))
  (Variables|Default|SetEstaleyendo false))

(event Custom|Toggle%20Pickup
  (if (Variables|Default|GetEstaleyendo)
    (CallFunction|PutDownNote)
    (else
      (CallFunction|PickupNote))))

(event Custom|PickupNote
  (bind _returnvalue (UserInterface|CreateWidget "/Game/Blueprints/BP_widgetDiario.BP_widgetDiario_C"))
  (UserInterface|Viewport|AddtoViewport _returnvalue 0)
  (Variables|Default|SetEstaleyendo true))

(event EventInteractuar
  (params (HitComponent :type Actor%20Component%20Object%20Reference))
  (CallFunction|TogglePickup))

(fn ConstructionScript)