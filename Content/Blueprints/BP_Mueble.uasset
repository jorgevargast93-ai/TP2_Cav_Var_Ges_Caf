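; BP_Mueble is an interactive piece of furniture with a drawer (Cajom) and a door (Puerta) that toggle open and closed.
; Interactuar checks the hit component, then a FlipFlop plays or reverses that part's timeline, sliding the drawer along relative Y or rotating the door in yaw.
; A Box overlap with BP_FirstPersonCharacter enables input and shows the InterfazInterraccion widget, and leaving disables input and removes it.
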(event OnComponentBeginOverlap(Box)
  (params (OverlappedComponent :type Primitive%20Component%20Object%20Reference) (OtherActor :type Actor%20Object%20Reference) (OtherComp :type Primitive%20Component%20Object%20Reference) (OtherBodyIndex :type Integer) (bFromSweep :type Boolean) (SweepResult :type Hit%20Result%20Structure%20%28by%20ref%29))
  (Utilities|Casting|CastToBP_FirstPersonCharacter OtherActor)
  (Input|EnableInput (Game|GetPlayerController 0))
  (bind _returnvalue (UserInterface|CreateWidget "/Game/Blueprints/InterfazInterraccion.InterfazInterraccion_C"))
  (UserInterface|Viewport|AddtoViewport _returnvalue 0))

(event OnComponentEndOverlap(Box)
  (params (OverlappedComponent :type Primitive%20Component%20Object%20Reference) (OtherActor :type Actor%20Object%20Reference) (OtherComp :type Primitive%20Component%20Object%20Reference) (OtherBodyIndex :type Integer))
  (Utilities|Casting|CastToBP_FirstPersonCharacter OtherActor)
  (Input|DisableInput 0)
  (Widget|RemovefromParent (stale OnComponentBeginOverlap(Box) _returnvalue)))

(event EventBeginPlay)

(event Collision|EventActorBeginOverlap
  (params (OtherActor :type Actor%20Object%20Reference)))

(event EventTick
  (params (DeltaSeconds :type Float%20%28single-precision%29)))

(event EventInteractuar
  (params (HitComponent :type Actor%20Component%20Object%20Reference))
  (if (== HitComponent (Variables|Default|Getcajom))
    (Utilities|FlowControl|FlipFlop
      (:A
        (bind _newtrack_3 (Timeline|MOVER_Y Play)
          (:Update
            (Transformation|SetRelativeLocation (Variables|Default|Getcajom) (Math|Vector|MakeVector 0.0 _newtrack_3 69.0) false false))))
      (:B
        (Timeline|MOVER_Y Reverse)))
    (elif (== HitComponent (Variables|Default|Getpuerta))
      (Utilities|FlowControl|FlipFlop
        (:A
          (bind _newtrack_0 (Timeline|rotacion Play)
            (:Update
              (Transformation|SetRelativeRotation (Variables|Default|Getpuerta) (Math|Rotator|MakeRotator 0.0 0.0 _newtrack_0) false false))))
        (:B
          (Timeline|rotacion Reverse))))))

(event Input|KeyboardEvents|E
  (params (Key :type Key%20Structure :default "None")))

(fn ConstructionScript)